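; Interactable puzzle chest that stays locked until unlocked, then toggles between open and closed sprites with matching sounds.
; Interacting while locked plays a stuck sound, zeroes the player's move speed and shows a WBP_Puzzle widget holding a reference to the chest.
; UnlockChest sets the unlocked state and runs the same toggle, while ClosePuzzle removes the widget and restores player speed and facing.
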(event Custom|Unlock%20Chest
  (bind _chest (Variables|Default|GetChest))
  (bind _defaultsceneroot (Variables|Default|GetDefaultSceneRoot))
  (bind _returnvalue (Transformation|GetWorldLocation _defaultsceneroot))
  (Variables|Default|SetUnlocked true)
  (bind _output_get (Variables|Default|SetIsOpen (not (Variables|Default|GetIsOpen))))
  (if (and _output_get (Variables|Default|GetUnlocked))
    ;[1 1 1] Open Chest
    (Audio|PlaySoundatLocation "/Game/Audio/SFX/01_chest_open_4.01_chest_open_4" _returnvalue "0, 0, 0" 1.0 1.0 0.0 0 0 0 0)
    (Rendering|Components|Sprite|SetSprite _chest "/Game/Assets/Sprites/ChestOpen.ChestOpen")
    (else
      ;[1 1 1] Close Chest
      (Audio|PlaySoundatLocation "/Game/Audio/SFX/02_chest_close_1.02_chest_close_1" _returnvalue "0, 0, 0" 1.0 1.0 0.0 0 0 0 0)
      (Rendering|Components|Sprite|SetSprite _chest "/Game/Assets/Sprites/ChestClosed.ChestClosed"))))

(event Custom|OpenChest
  (bind _chest (Variables|Default|GetChest))
  (bind _defaultsceneroot (Variables|Default|GetDefaultSceneRoot))
  (bind _returnvalue (Transformation|GetWorldLocation _defaultsceneroot))
  (bind _output_get (Variables|Default|SetIsOpen (not (Variables|Default|GetIsOpen))))
  (if (and _output_get (Variables|Default|GetUnlocked))
    ;[1 1 1] Open Chest
    (Audio|PlaySoundatLocation "/Game/Audio/SFX/01_chest_open_4.01_chest_open_4" _returnvalue "0, 0, 0" 1.0 1.0 0.0 0 0 0 0)
    (Rendering|Components|Sprite|SetSprite _chest "/Game/Assets/Sprites/ChestOpen.ChestOpen")
    (else
      ;[1 1 1] Close Chest
      (Audio|PlaySoundatLocation "/Game/Audio/SFX/02_chest_close_1.02_chest_close_1" _returnvalue "0, 0, 0" 1.0 1.0 0.0 0 0 0 0)
      (Rendering|Components|Sprite|SetSprite _chest "/Game/Assets/Sprites/ChestClosed.ChestClosed"))))

(event EventBeginPlay)

(event Collision|EventActorBeginOverlap
  (params (OtherActor :type Actor%20Object%20Reference)))

(event EventTick
  (params (DeltaSeconds :type Float%20%28single-precision%29)))

(event EventInteractwith
  (bind _chest (Variables|Default|GetChest))
  (bind _defaultsceneroot (Variables|Default|GetDefaultSceneRoot))
  (bind _returnvalue (Transformation|GetWorldLocation _defaultsceneroot))
  (if (Variables|Default|GetUnlocked)
    (bind _output_get (Variables|Default|SetIsOpen (not (Variables|Default|GetIsOpen))))
    (if (and _output_get (Variables|Default|GetUnlocked))
      ;[1 1 1] Open Chest
      (Audio|PlaySoundatLocation "/Game/Audio/SFX/01_chest_open_4.01_chest_open_4" _returnvalue "0, 0, 0" 1.0 1.0 0.0 0 0 0 0)
      (Rendering|Components|Sprite|SetSprite _chest "/Game/Assets/Sprites/ChestOpen.ChestOpen")
      (else
        ;[1 1 1] Close Chest
        (Audio|PlaySoundatLocation "/Game/Audio/SFX/02_chest_close_1.02_chest_close_1" _returnvalue "0, 0, 0" 1.0 1.0 0.0 0 0 0 0)
        (Rendering|Components|Sprite|SetSprite _chest "/Game/Assets/Sprites/ChestClosed.ChestClosed")))
    (elif (not (Variables|Default|GetIsBeingExamined))
      ;[1 1 1] Chest Stuck Sound
      (Audio|PlaySoundatLocation "/Game/Audio/SFX/02_chest_close_3.02_chest_close_3" _returnvalue "0, 0, 0" 1.0 1.0 0.0 0 0 0 0)
      (Variables|Default|SetIsBeingExamined true)
      (CallFunction|SetupPuzzle))))

(fn ConstructionScript)

(fn SetupPuzzle
  (bind _asbp_top_down_char (Utilities|Casting|CastToBP_TopDownChar (Game|Player|GetPlayerPawn 0)))
  (Variables|/Game/Character/BP_TopDownChar.BP_TopDownChar_C|SetMoveSpeed _asbp_top_down_char 0.0)
  (bind _returnvalue (UserInterface|CreateWidget "/Game/Widgets/WBP_Puzzle.WBP_Puzzle_C" 0 self))
  (bind _output_get (Variables|Default|SetPuzzleWidget _returnvalue))
  (UserInterface|Viewport|AddtoViewport _output_get 0))

(fn ClosePuzzle
  (bind _asbp_top_down_char (Utilities|Casting|CastToBP_TopDownChar (Game|Player|GetPlayerPawn 0)))
  (Variables|/Game/Character/BP_TopDownChar.BP_TopDownChar_C|SetMoveSpeed _asbp_top_down_char 0.15)
  (Variables|/Game/Character/BP_TopDownChar.BP_TopDownChar_C|SetDirectionality _asbp_top_down_char "(X=0.000000,Y=1.000000)")
  (Variables|Default|SetIsBeingExamined false)
  (Widget|RemovefromParent (Variables|Default|GetPuzzleWidget)))