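; BP_RoomManager moves the player between rooms and runs timed damage in the combat level.
; When the player character overlaps its box, it opens a random level from a hard-coded start, puzzle and combat list.
; Tick shows the UserTyped widget only in Level_Combat while player and enemy health, both read from BP_TopDownChar, remain above zero.
; In that state, a Delay on Tick damages the player roughly every five seconds.
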(event OnComponentBeginOverlap(Box)
  (params (OverlappedComponent :type Primitive%20Component%20Object%20Reference) (OtherActor :type Actor%20Object%20Reference) (OtherComp :type Primitive%20Component%20Object%20Reference) (OtherBodyIndex :type Integer) (bFromSweep :type Boolean) (SweepResult :type Hit%20Result%20Structure%20%28by%20ref%29))
  (Utilities|Casting|CastToBP_TopDownChar OtherActor)
  (bind _output_get (Variables|Default|SetLevels (Utilities|Array|MakeArray "Level_Start" "Level_Puzzle1" "Level_Combat")))
  (Game|OpenLevel(byName) (.OutItem (Utilities|Array|Random _output_get))))

(event EventBeginPlay
  (bind _returnvalue (UserInterface|CreateWidget "/Game/Widgets/UserTyped.UserTyped_C"))
  (bind _output_get (Variables|Default|SetUserTypedRef _returnvalue))
  (UserInterface|Viewport|AddtoViewport _output_get 0)
  (Widget|SetVisibility _output_get "Visible")
  (bind _asbp_top_down_char (Utilities|Casting|CastToBP_TopDownChar (Game|Player|GetPlayerPawn 0)))
  (Variables|Default|SetTopDownCharRef _asbp_top_down_char))

(event Collision|EventActorBeginOverlap
  (params (OtherActor :type Actor%20Object%20Reference)))

(event EventTick
  (params (DeltaSeconds :type Float%20%28single-precision%29))
  (bind _topdowncharref (Variables|Default|GetTopDownCharRef))
  (bind _usertypedref (Variables|Default|GetUserTypedRef))
  (if (or (<= (Variables|/Game/Character/BP_TopDownChar.BP_TopDownChar_C|GetHealth _topdowncharref) 0.0) (<= (Variables|/Game/Character/BP_TopDownChar.BP_TopDownChar_C|GetEnemyHealth _topdowncharref) 0.0))
    (Widget|SetVisibility (Variables|Default|GetUserTypedRef) "Hidden")
    (else
      (bind _returnvalue (Game|GetCurrentLevelName true))
      (if (Utilities|Enum|Equal(Enum) _returnvalue "Level_Combat")
        (Widget|SetVisibility _usertypedref "Visible")
        (Utilities|FlowControl|Delay 5.0)
        (Game|Damage|ApplyDamage (Variables|Default|GetTopDownCharRef) 5.0 0 0)
        (else
          (Widget|SetVisibility _usertypedref "Hidden"))))))

(fn ConstructionScript)