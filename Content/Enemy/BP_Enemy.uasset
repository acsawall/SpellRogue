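; Enemy actor Blueprint that damages the top-down player character after an overlap begins.
; BeginPlay initializes EnemyHealth, which is not used elsewhere in the file.
; Any overlap starts a delay, then DealPlayerDamage casts player pawn 0 to BP_TopDownChar and subtracts a random amount from its Health.
; The returned Health gates a loop back to the delay, repeating only while it equals zero.
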(event EventBeginPlay
  (Variables|Default|SetEnemyHealth 100))

(event Collision|EventActorBeginOverlap
  (params (OtherActor :type Actor%20Object%20Reference))
  (Utilities|FlowControl|Delay 15.0 :!label _label)
  (bind _currplayerhealth (CallFunction|DealPlayerDamage))
  (while (== _currplayerhealth 0)
    (goto _label)))

(event EventTick
  (params (DeltaSeconds :type Float%20%28single-precision%29)))

(fn ConstructionScript)

(fn DealPlayerDamage
  (bind _asbp_top_down_char (Utilities|Casting|CastToBP_TopDownChar (Game|Player|GetPlayerPawn 0)))
  (bind _output_get (Variables|/Game/Character/BP_TopDownChar.BP_TopDownChar_C|SetHealth _asbp_top_down_char (- (Variables|/Game/Character/BP_TopDownChar.BP_TopDownChar_C|GetHealth _asbp_top_down_char) (Math|Random|RandomInteger 30))))
  (return _output_get))