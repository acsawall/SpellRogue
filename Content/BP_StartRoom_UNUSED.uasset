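; Start room Blueprint, marked unused, for a top-down Paper2D dungeon with overlap triggers for a chest, door and lever that respond to BP_TopDownChar.
; The lever toggles RoomComplete and sets its flipped tiles, and the door trigger opens the door only while that flag is true.
; Door and lever visuals are swapped by editing the tile map at runtime, with collision rebuilt for doors.
; OpenChest is an empty stub, and CloseDoor is never called here.
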(event OnComponentBeginOverlap(ChestCollider)
  (params (OverlappedComponent :type Primitive%20Component%20Object%20Reference) (OtherActor :type Actor%20Object%20Reference) (OtherComp :type Primitive%20Component%20Object%20Reference) (OtherBodyIndex :type Integer) (bFromSweep :type Boolean) (SweepResult :type Hit%20Result%20Structure%20%28by%20ref%29))
  (Utilities|Casting|CastToBP_TopDownChar OtherActor)
  (CallFunction|OpenChest))

(event OnComponentBeginOverlap(DoorCollider)
  (params (OverlappedComponent :type Primitive%20Component%20Object%20Reference) (OtherActor :type Actor%20Object%20Reference) (OtherComp :type Primitive%20Component%20Object%20Reference) (OtherBodyIndex :type Integer) (bFromSweep :type Boolean) (SweepResult :type Hit%20Result%20Structure%20%28by%20ref%29))
  (Utilities|Casting|CastToBP_TopDownChar OtherActor)
  (if (Variables|Default|GetRoomComplete)
    (CallFunction|OpenDoor)))

(event OnComponentBeginOverlap(LeverCollider)
  (params (OverlappedComponent :type Primitive%20Component%20Object%20Reference) (OtherActor :type Actor%20Object%20Reference) (OtherComp :type Primitive%20Component%20Object%20Reference) (OtherBodyIndex :type Integer) (bFromSweep :type Boolean) (SweepResult :type Hit%20Result%20Structure%20%28by%20ref%29))
  (bind _asbp_top_down_char (Utilities|Casting|CastToBP_TopDownChar OtherActor))
  (if (Collision|IsOverlappingActor (Variables|Default|GetLeverCollider) _asbp_top_down_char :!class /Script/Engine.PrimitiveComponent)
    (CallFunction|FlipLever 11 3 4)))

(event EventBeginPlay)

(event Collision|EventActorBeginOverlap
  (params (OtherActor :type Actor%20Object%20Reference)))

(event EventTick
  (params (DeltaSeconds :type Float%20%28single-precision%29)))

(fn ConstructionScript)

(fn OpenDoor
  (bind _papertilemap (Variables|Default|GetPaperTileMap))
  (bind _papertilemap_2 (Variables|Default|GetPaperTileMap))
  (Class|PaperTileMapComponent|MakeTileMapEditable _papertilemap_2)
  (bind _mapwidth (Class|PaperTileMapComponent|GetMapSize _papertilemap_2))
  ;[1 1 1] Right Door
  (Class|PaperTileMapComponent|SetTile _papertilemap (/ _mapwidth 2) 0 3 (Class|TileMapBlueprintLibrary|MakeTile 48 "/Game/Assets/TileSets/Dungeon_Tileset.Dungeon_Tileset"))
  ;[1 1 1] Left Door
  (Class|PaperTileMapComponent|SetTile _papertilemap (- (/ _mapwidth 2) 1) 0 3 (Class|TileMapBlueprintLibrary|MakeTile 47 "/Game/Assets/TileSets/Dungeon_Tileset.Dungeon_Tileset"))
  (Class|PaperTileMapComponent|RebuildCollision (Variables|Default|GetPaperTileMap)))

(fn OpenChest)

(fn CloseDoor
  (bind _papertilemap (Variables|Default|GetPaperTileMap))
  (bind _papertilemap_2 (Variables|Default|GetPaperTileMap))
  (Class|PaperTileMapComponent|MakeTileMapEditable _papertilemap_2)
  (bind _mapwidth (Class|PaperTileMapComponent|GetMapSize _papertilemap_2))
  ;[1 1 1] Right Door
  (Class|PaperTileMapComponent|SetTile _papertilemap (/ _mapwidth 2) 0 3 (Class|TileMapBlueprintLibrary|MakeTile 37 "/Game/Assets/TileSets/Dungeon_Tileset.Dungeon_Tileset"))
  ;[1 1 1] Left Door
  (Class|PaperTileMapComponent|SetTile _papertilemap (- (/ _mapwidth 2) 1) 0 3 (Class|TileMapBlueprintLibrary|MakeTile 36 "/Game/Assets/TileSets/Dungeon_Tileset.Dungeon_Tileset"))
  (Class|PaperTileMapComponent|RebuildCollision (Variables|Default|GetPaperTileMap)))

(fn FlipLever
  (params (LeverX :type Integer) (LeverY1 :type Integer) (LeverY2 :type Integer))
  (bind _papertilemap (Variables|Default|GetPaperTileMap))
  (Variables|Default|SetRoomComplete (not (Variables|Default|GetRoomComplete)))
  (Class|PaperTileMapComponent|MakeTileMapEditable (Variables|Default|GetPaperTileMap))
  (Class|PaperTileMapComponent|SetTile _papertilemap LeverX LeverY1 2 (Class|TileMapBlueprintLibrary|MakeTile 181 "/Game/Assets/TileSets/Props_TileSet.Props_TileSet"))
  (Class|PaperTileMapComponent|SetTile _papertilemap LeverX LeverY2 2 (Class|TileMapBlueprintLibrary|MakeTile 206 "/Game/Assets/TileSets/Props_TileSet.Props_TileSet")))