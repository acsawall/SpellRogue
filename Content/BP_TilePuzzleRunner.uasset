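; Runs a letter-tile spelling puzzle that unlocks the level's BP_Chest when the word is completed.
; On BeginPlay it picks a random string-table key as the word, scatters one BP_Letter per character within PuzzleBounds, and assigns sprites by matching PrimaryAssetId names.
; SolvePiece hides each tile hit in the correct order and trims the remaining solution.
; A wrong letter calls ResetPuzzle, which re-shows and re-letters the existing tiles.
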(event Custom|Solve%20Piece
  (params (Letter :type String) (Piece%20Object :type BP%20Letter%20Object%20Reference))
  ;[1 1 1] If the letter was the next step in the solution
  (if (Utilities|Enum|Equal(Enum) Letter (Utilities|String|GetSubstring (Variables|Default|GetSolution%20Progress) 0))
    ;[1 1 1] Disable the piece
    (Variables|/Script/Engine.PrimitiveComponent|SetbGenerateOverlapEvents (Actor|GetComponentbyClass Piece%20Object "/Script/Engine.BoxComponent") false)
    (Rendering|SetActorHiddenInGame Piece%20Object true)
    ;[1 1 1] Remove the solved character
    (bind _output_get (Variables|Default|SetSolution%20Progress (Utilities|String|GetSubstring (Variables|Default|GetSolution%20Progress) 1 (- (Utilities|String|Len (Variables|Default|GetSolution%20Progress)) 1))))
    ;[1 1 1] If solution completely solved
    (if (== (Utilities|String|Len _output_get) 0)
      (Utilities|FlowControl|DoOnce false
        (:Completed
          (Variables|Default|SetSolved true)
          (Development|PrintString "Solved!")
          (CallFunction|TryUnlockChest))))
    (else
      (CallFunction|ResetPuzzle))))

(event EventBeginPlay
  (bind _puzzlebounds (Variables|Default|GetPuzzleBounds))
  (bind (_origin _boxextent) (Collision|GetComponentBounds _puzzlebounds))
  ;[1 1 1] select random word
  (bind _output_get (Variables|Default|SetWord (.OutItem (Utilities|Array|Random (Class|KismetStringTableLibrary|GetKeysfromStringTable "/Game/PuzzleWords.PuzzleWords")))))
  (Variables|Default|SetSolution%20Progress (Variables|Default|GetWord))
  (for _index (range 0 (- (Utilities|String|Len _output_get) 1))
    (bind _returnvalue (Game|SpawnActorfromClass "/Game/Assets/Interactables/BP_Letter.BP_Letter_C" (Math|Transform|MakeTransform (Math|Vector|MakeVector (+ (.x _origin) (Math|Random|RandomFloatinRange (* -1.0 (.x _boxextent)) (.x _boxextent))) (+ (.y _origin) (Math|Random|RandomFloatinRange (* -1.0 (.y _boxextent)) (.y _boxextent))) 1.0) "0, 0, 0" "1.000000,1.000000,1.000000") "AdjustIfPossibleButAlwaysSpawn" "MultiplyWithRoot" 0 0))
    ;[1 1 1] reset all Letters to blank
    (Rendering|Components|Sprite|SetSprite (Variables|/Game/Assets/Interactables/BP_Letter.BP_Letter_C|GetLetter _returnvalue) "/Game/Assets/Sprites/Letters/space.space")
    ;[1 1 1] Enable all letter objects
    (Variables|/Script/Engine.PrimitiveComponent|SetbGenerateOverlapEvents (Actor|GetComponentbyClass _returnvalue "/Script/Engine.BoxComponent") true)
    (Rendering|SetActorHiddenInGame _returnvalue false))
  ;[1 1 1] For each solution letter
  (bind _output_get_2 (Variables|Default|SetSolution%20Buff%20Arr (Utilities|String|GetCharacterArrayfromString (Variables|Default|GetWord))))
  (for _array_element _output_get_2
    (bind _outactors (Actor|GetAllActorsOfClass "/Game/Assets/Interactables/BP_Letter.BP_Letter_C"))
    ;[1 1 1] find an empty letter
    (bind _array_element_2 (Utilities|Array|ForEachLoopwithBreak _outactors :!label _label)
      (:LoopBody
        (if (Utilities|Enum|Equal(Enum) (Utilities|GetObjectName (Sprite|GetSprite (Variables|/Game/Assets/Interactables/BP_Letter.BP_Letter_C|GetLetter _array_element_2))) "space")
          (goto _label Break)))
      (:Completed
        ;[1 1 1] find the correct sprite to assign
        (bind _outprimaryassetidlist (Class|KismetSystemLibrary|GetPrimaryAssetIdList "PaperSprite"))
        (bind _array_element_3 (Utilities|Array|ForEachLoopwithBreak _outprimaryassetidlist :!label _label_2)
          (:LoopBody
            (if (Utilities|Enum|Equal(Enum) (Utilities|String|ToString(Integer) _array_element_3) (Utilities|String|Append "PaperSprite:" _array_element))
              (goto _label_2 Break)))
          (:Completed
            ;[1 1 1] Load sprite
            (bind _returnvalue_2 (Utilities|LoadAssetBlocking (Class|KismetSystemLibrary|GetSoftObjectReferencefromPrimaryAssetId _array_element_3)))
            (bind _aspaper_sprite (Utilities|Casting|CastToPaperSprite _returnvalue_2))
            (Default|SetLetter _array_element_2 _aspaper_sprite)))))))

(fn ConstructionScript)

(fn ResetPuzzle
  (Variables|Default|SetSolution%20Progress (Variables|Default|GetWord))
  (bind _outactors (Actor|GetAllActorsOfClass "/Game/Assets/Interactables/BP_Letter.BP_Letter_C"))
  ;[1 1 1] reset all Letters to blank
  (for _array_element _outactors
    (Rendering|Components|Sprite|SetSprite (Variables|/Game/Assets/Interactables/BP_Letter.BP_Letter_C|GetLetter _array_element) "/Game/Assets/Sprites/Letters/space.space")
    ;[1 1 1] Enable all letter objects
    (Variables|/Script/Engine.PrimitiveComponent|SetbGenerateOverlapEvents (Actor|GetComponentbyClass _array_element "/Script/Engine.BoxComponent") true)
    (Rendering|SetActorHiddenInGame _array_element false))
  ;[1 1 1] For each solution letter
  (bind _output_get (Variables|Default|SetSolution%20Buff%20Arr (Utilities|String|GetCharacterArrayfromString (Variables|Default|GetWord))))
  (for _array_element_2 _output_get
    (bind _outactors_2 (Actor|GetAllActorsOfClass "/Game/Assets/Interactables/BP_Letter.BP_Letter_C"))
    ;[1 1 1] find an empty letter
    (bind _array_element_3 (Utilities|Array|ForEachLoopwithBreak _outactors_2 :!label _label)
      (:LoopBody
        (if (Utilities|Enum|Equal(Enum) (Utilities|GetObjectName (Sprite|GetSprite (Variables|/Game/Assets/Interactables/BP_Letter.BP_Letter_C|GetLetter _array_element_3))) "space")
          (goto _label Break)))
      (:Completed
        ;[1 1 1] find the correct sprite to assign
        (bind _outprimaryassetidlist (Class|KismetSystemLibrary|GetPrimaryAssetIdList "PaperSprite"))
        (bind _array_element_4 (Utilities|Array|ForEachLoopwithBreak _outprimaryassetidlist :!label _label_2)
          (:LoopBody
            (if (Utilities|Enum|Equal(Enum) (Utilities|String|ToString(Integer) _array_element_4) (Utilities|String|Append "PaperSprite:" _array_element_2))
              (goto _label_2 Break)))
          (:Completed
            ;[1 1 1] Load sprite
            (bind _returnvalue (Utilities|LoadAssetBlocking (Class|KismetSystemLibrary|GetSoftObjectReferencefromPrimaryAssetId _array_element_4)))
            (bind _aspaper_sprite (Utilities|Casting|CastToPaperSprite _returnvalue))
            (Default|SetLetter _array_element_3 _aspaper_sprite)))))))

(fn TryUnlockChest
  (bind _returnvalue (Actor|GetActorOfClass "/Game/Assets/Interactables/BP_Chest.BP_Chest_C"))
  (Default|UnlockChest _returnvalue))