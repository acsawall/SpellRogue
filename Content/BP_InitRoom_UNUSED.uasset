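; An unused, unfinished Blueprint that sets up a dungeon room on a Paper2D tile map at runtime.
; BeginPlay makes the map editable, reads its size, then runs a placeholder single-pass loop for top and bottom walls, with no tile value specified.
; Map creation, corner-wall placement from the dungeon tileset and collision rebuilding are disconnected and never run.
; GetAttachTransform exposes the AttachPoint's world transform.
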(event EventBeginPlay
  (bind _emptytilemap (Variables|Default|GetEmptyTileMap))
  (bind _emptytilemap_2 (Variables|Default|GetEmptyTileMap))
  (bind _tilemap (Variables|/Script/Paper2D.PaperTileMapComponent|GetTileMap _emptytilemap))
  (Class|PaperTileMapComponent|MakeTileMapEditable _emptytilemap)
  (Variables|Default|SetMapWidth (Variables|/Script/Paper2D.PaperTileMap|GetMapWidth _tilemap))
  (Variables|Default|SetMapHeight (Variables|/Script/Paper2D.PaperTileMap|GetMapHeight _tilemap))
  ;[1 1 1] Top and Bottom Walls
  (for _index (range 0 0)
    (Class|PaperTileMapComponent|SetTile _emptytilemap_2 _index 0 3)
    (Class|PaperTileMapComponent|SetTile _emptytilemap_2 _index 0 3)))

(event Collision|EventActorBeginOverlap
  (params (OtherActor :type Actor%20Object%20Reference)))

(event EventTick
  (params (DeltaSeconds :type Float%20%28single-precision%29)))

(fn ConstructionScript)

(fn GetAttachTransform
  (return (Transformation|GetWorldTransform (Variables|Default|GetAttach%20Point))))